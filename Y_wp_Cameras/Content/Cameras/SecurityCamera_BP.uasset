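; Destructible networked security camera that sweeps, tracks players and renders its view to a render target.
; On authority, a timeline drives the idle sweep, and a trigger overlap locks onto a FirstPersonCharacter with clamped, interpolated rotation; remotes drop tick, capture and trigger.
; ManualControl suspends automatic movement, with events exposed for pan, tilt and zoom.
; Lethal damage stops it, removes its components, starts smoke and notifies the owning terminal.
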(event OnComponentBeginOverlap(ViewTrigger)
  (params (OverlappedComponent :type Primitive%20Component%20Object%20Reference) (OtherActor :type Actor%20Object%20Reference) (OtherComp :type Primitive%20Component%20Object%20Reference) (OtherBodyIndex :type Integer) (bFromSweep :type Boolean) (SweepResult :type Hit%20Result%20Structure%20%28by%20ref%29))
  ;[1 1 1] Setting target
  (Networking|SwitchHasAuthority
    (:Authority
      (if (not (Variables|Default|GetHasTarget))
        (bind _asfirst_person_character (Utilities|Casting|CastToFirstPersonCharacter OtherActor))
        (Variables|Default|SetTargetActor _asfirst_person_character)
        (Variables|Default|SetHasTarget true)))))

(event OnComponentEndOverlap(ViewTrigger)
  (params (OverlappedComponent :type Primitive%20Component%20Object%20Reference) (OtherActor :type Actor%20Object%20Reference) (OtherComp :type Primitive%20Component%20Object%20Reference) (OtherBodyIndex :type Integer))
  ;[1 1 1] Setting target
  (Networking|SwitchHasAuthority
    (:Authority
      (if (and (== OtherActor (Variables|Default|GetTargetActor)) (Variables|Default|GetHasTarget))
        (Variables|Default|SetHasTarget false)
        (Variables|Default|SetTargetActor 0)))))

(event Custom|AddYawRotation
  (params (Value :type Float%20%28single-precision%29))
  (bind _camera (Variables|Default|GetCamera))
  (bind _relativerotation (Variables|/Script/Engine.SceneComponent|GetRelativeRotation _camera))
  ;[1 1 1] Player Controls
  (Transformation|SetRelativeRotation (Variables|Default|GetCamera) (Math|Rotator|MakeRotator 0.0 (.pitch _relativerotation) (Math|Float|ClampAngle (+ (.yaw _relativerotation) Value) (* (Variables|Default|GetCameraSearchAngle) -1.0) (Variables|Default|GetCameraSearchAngle))) false false))

(event Custom|AddPitchRotation
  (params (Value :type Float%20%28single-precision%29))
  (bind _camera (Variables|Default|GetCamera))
  (bind _relativerotation (Variables|/Script/Engine.SceneComponent|GetRelativeRotation _camera))
  ;[1 1 1] Player Controls
  (Transformation|SetRelativeRotation (Variables|Default|GetCamera) (Math|Rotator|MakeRotator 0.0 (Math|Float|ClampAngle (- (.pitch _relativerotation) Value) -8e+01 8e+01) (.yaw _relativerotation)) false false))

(event Custom|AddCameraFOV
  (params (Value :type Float%20%28single-precision%29))
  ;[1 1 1] Player Controls
  (Variables|/Script/Engine.SceneCaptureComponent2D|SetFOVAngle (Variables|Default|GetSceneCaptureComponent2D) (Math|Float|Clamp(Float) (- (Variables|/Script/Engine.SceneCaptureComponent2D|GetFOVAngle (Variables|Default|GetSceneCaptureComponent2D)) Value) 25.0 1e+02)))

(event Custom|ResetFOV
  (bind _scenecapturecomponent2d (Variables|Default|GetSceneCaptureComponent2D))
  ;[1 1 1] Player Controls
  (Variables|/Script/Engine.SceneCaptureComponent2D|SetFOVAngle _scenecapturecomponent2d (Math|Interpolation|FInterpTo (Variables|/Script/Engine.SceneCaptureComponent2D|GetFOVAngle (Variables|Default|GetSceneCaptureComponent2D)) (Variables|Default|GetDefaultFOV) (Utilities|Time|GetWorldDeltaSeconds) 5.0) :!label _label)
  (Utilities|FlowControl|Delay (Utilities|Time|GetWorldDeltaSeconds))
  (Utilities|IsValid _scenecapturecomponent2d
    (:Is%20Valid
      (if (not (and (Variables|Default|GetManualControl) (Math|Float|NearlyEqual(Float) (Variables|/Script/Engine.SceneCaptureComponent2D|GetFOVAngle (Variables|Default|GetSceneCaptureComponent2D)) (Variables|Default|GetDefaultFOV) 0.005)))
        (goto _label)))))

(event Custom|StopTimeline
  ;[1 1 1] Idle Movement
  (bind _cammovement (Timeline|CameraIdleRotation Stop)
    (:Update
      (Variables|Default|SetNewRotation (Math|Rotator|Lerp(Rotator) (Math|Rotator|MakeRotator 0.0 (Variables|Default|GetCameraPitch) (Variables|Default|GetCameraSearchAngle)) (Math|Rotator|MakeRotator 0.0 (Variables|Default|GetCameraPitch) (* (Variables|Default|GetCameraSearchAngle) -1.0)) _cammovement)))))

(event Custom|MC_DestroyCamera
  ;[1 1 1] Take Damage And Destroyed
  (Components|DestroyComponent (Variables|Default|GetCamera))
  (Components|Activation|SetActive (Variables|Default|GetP_Smoke) true false))

(event Custom|Event_Destroyed
  ;[1 1 1] Take Damage And Destroyed
  (Variables|Default|SetIsDestroyed true)
  (CallFunction|StopTimeline)
  (Actor|Tick|SetActorTickEnabled false)
  (CallFunction|MCDestroyCamera)
  (Components|DestroyComponent (Variables|Default|GetSceneCaptureComponent2D))
  (Default|CameraDestroyed (Variables|Default|GetOwningTerminal) self))

(event EventBeginPlay
  ;[1 1 1] Idle Movement
  (Networking|SwitchHasAuthority
    (:Authority
      (bind _cammovement (Timeline|CameraIdleRotation PlayFromStart)
        (:Update
          (Variables|Default|SetNewRotation (Math|Rotator|Lerp(Rotator) (Math|Rotator|MakeRotator 0.0 (Variables|Default|GetCameraPitch) (Variables|Default|GetCameraSearchAngle)) (Math|Rotator|MakeRotator 0.0 (Variables|Default|GetCameraPitch) (* (Variables|Default|GetCameraSearchAngle) -1.0)) _cammovement)))))))

(event EventTakeDamage
  (params (Amount :type Float%20%28single-precision%29))
  ;[1 1 1] Take Damage And Destroyed
  (if (not (Variables|Default|GetIsDestroyed))
    (bind _output_get (Variables|Default|SetHealth (- (Variables|Default|GetHealth) Amount)))
    (if (<= _output_get 0.0)
      (CallFunction|EventDestroyed))))

(event EventTick
  (params (DeltaSeconds :type Float%20%28single-precision%29))
  (bind _camera (Variables|Default|GetCamera))
  (bind _targetactor (Variables|Default|GetTargetActor))
  (bind _returnvalue (Transformation|GetWorldRotation _camera))
  (bind _returnvalue_2 (Transformation|GetWorldLocation _camera))
  (bind _returnvalue_3 (Transformation|GetActorLocation _targetactor))
  (bind _returnvalue_4 (Math|Rotator|GetRotationXVector _returnvalue))
  (bind _returnvalue_5 (Math|Vector|GetUnitDirection(Vector) _returnvalue_2 _returnvalue_3))
  (bind _returnvalue_6 (Math|Interpolation|VInterpTo _returnvalue_4 _returnvalue_5 DeltaSeconds 6.0))
  (bind _returnvalue_7 (Math|Rotator|MakeRotfromX _returnvalue_6))
  (bind (_roll _pitch _yaw) (Math|Rotator|BreakRotator _returnvalue_7))
  ;[1 1 1] Idle Movement
  (if (not (Variables|Default|GetManualControl))
    (Networking|SwitchHasAuthority
      (:Authority
        (if (Variables|Default|GetHasTarget)
          ;[1 1 1] Follow Target
          (Transformation|SetWorldRotation (Variables|Default|GetCamera) (Math|Rotator|MakeRotator 0.0 (Math|Float|ClampAngle _pitch (Variables|Default|GetCam_MinPitch) (Variables|Default|GetCam_MaxPitch)) (Math|Float|ClampAngle _yaw (Variables|Default|GetCam_MinYaw) (Variables|Default|GetCam_MaxYaw))) false false)
          (else
            (Transformation|SetRelativeRotation (Variables|Default|GetCamera) (Math|Interpolation|RInterpTo (Variables|/Script/Engine.SceneComponent|GetRelativeRotation (Variables|Default|GetCamera)) (Variables|Default|GetNewRotation) DeltaSeconds 0.3) false false))))
      (:Remote
        (Actor|Tick|SetActorTickEnabled false)
        (Components|DestroyComponent (Variables|Default|GetSceneCaptureComponent2D))))))

(fn ConstructionScript
  (bind _returnvalue (Math|Float|MakeLiteralFloat 8e+01))
  (bind _camera (Variables|Default|GetCamera))
  (bind _camerasearchangle (Variables|Default|GetCameraSearchAngle))
  (bind _returnvalue_2 (Transformation|GetWorldRotation _camera))
  (bind (_roll _pitch _yaw) (Math|Rotator|BreakRotator _returnvalue_2))
  ;[1 1 1] Set min/max angles
  (Variables|Default|SetCam_MinPitch (- _pitch _returnvalue))
  (Variables|Default|SetCam_MaxPitch (+ _pitch _returnvalue))
  (Variables|Default|SetCam_MinYaw (- _yaw _camerasearchangle))
  (Variables|Default|SetCam_MaxYaw (+ _yaw _camerasearchangle))
  ;[1 1 1] Apply pitch
  (Transformation|AddRelativeRotation (Variables|Default|GetCamera) (Math|Rotator|MakeRotator 0.0 (Variables|Default|GetCameraPitch) 0.0) false false)
  ;[1 1 1] Set default FOV
  (Variables|Default|SetDefaultFOV (Variables|/Script/Engine.SceneCaptureComponent2D|GetFOVAngle (Variables|Default|GetSceneCaptureComponent2D)))
  ;[1 1 1] Set RederTarget
  (Variables|/Script/Engine.SceneCaptureComponent2D|SetTextureTarget (Variables|Default|GetSceneCaptureComponent2D) (Variables|Default|GetTextureRenderTarget)))