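; Networked security terminal that lets one player at a time view and cycle through linked security cameras.
; The server handles trigger-based interaction, toggles scene captures and updates the user's UI directly or via client calls.
; While in use, captures switch to a UI render target, same-group screens follow, and other terminals' triggers are moved far below to disable them.
; Destroyed cameras show an offline screen and material.
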(event OnComponentBeginOverlap(Box)
  (params (OverlappedComponent :type Primitive%20Component%20Object%20Reference) (OtherActor :type Actor%20Object%20Reference) (OtherComp :type Primitive%20Component%20Object%20Reference) (OtherBodyIndex :type Integer) (bFromSweep :type Boolean) (SweepResult :type Hit%20Result%20Structure%20%28by%20ref%29))
  ;[1 1 1] Trigger Overlap events
  (if (Networking|IsServer)
    (bind _asfirst_person_character (Utilities|Casting|CastToFirstPersonCharacter OtherActor))
    (Variables|/Game/Blueprints/FirstPersonCharacter.FirstPersonCharacter_C|SetInteractableActor _asfirst_person_character self)
    (Utilities|Array|AddUnique (Variables|Default|GetAllPlayersInTrigger) _asfirst_person_character)
    (CallFunction|UIShowHint _asfirst_person_character true)))

(event OnComponentEndOverlap(Box)
  (params (OverlappedComponent :type Primitive%20Component%20Object%20Reference) (OtherActor :type Actor%20Object%20Reference) (OtherComp :type Primitive%20Component%20Object%20Reference) (OtherBodyIndex :type Integer))
  ;[1 1 1] Trigger Overlap events
  (if (Networking|IsServer)
    (bind _asfirst_person_character (Utilities|Casting|CastToFirstPersonCharacter OtherActor))
    (Variables|/Game/Blueprints/FirstPersonCharacter.FirstPersonCharacter_C|SetInteractableActor _asfirst_person_character 0)
    (Utilities|Array|RemoveItem (Variables|Default|GetAllPlayersInTrigger) _asfirst_person_character)
    (CallFunction|UIShowHint _asfirst_person_character false)))

(event Custom|MC_SetScreenMaterial
  (params (IsOffline :type Boolean))
  ;[1 1 1] SetScreenMaterial Multicast
  (if IsOffline
    (Rendering|Material|SetMaterial (Variables|Default|GetCube) 0 "/Game/Cameras/CamOffline_Mat.CamOffline_Mat")
    (else
      (Rendering|Material|SetMaterial (Variables|Default|GetCube) 0 (Variables|Default|GetScreenMaterialInstance)))))

(event Custom|ExitTerminal
  ;[1 1 1] Exit Terminal
  (if (Networking|IsServer)
    (Variables|Default|SetIsInUse false)
    (Variables|Default|SetUser_PlayerController 0)
    (CallFunction|UIShowAllHints true)
    (CallFunction|SetUIRendertarget false)
    (CallFunction|DisableAllOtherTerminals false)
    (else
      (Development|PrintString "ERROR: Client interaction" true true "(R=1.000000,G=0.000000,B=0.000000,A=1.000000)" 2e+01))))

(event Custom|CameraDestroyed
  (params (CameraBP :type Security%20Camera%20BP%20Object%20Reference))
  (bind _camera_bp (Variables|Default|GetCamera_BP))
  (bind _user_playercontroller (Variables|Default|GetUser_PlayerController))
  (bind _returnvalue (Utilities|Array|FindItem _camera_bp CameraBP))
  ;[1 1 1] Set propper screen materiials when a camera is destroyed
  (if (and (>= _returnvalue 0) (== _returnvalue (Variables|Default|GetCurrentIndex)))
    (Variables|Default|SetIsCurrentCamOffline true)
    (CallFunction|MCSetScreenMaterial (Variables|Default|GetIsCurrentCamOffline))
    (if (Variables|Default|GetIsInUse)
      (if (Pawn|IsLocalPlayerController _user_playercontroller)
        (Default|ShowOfflineScreen _user_playercontroller (Variables|Default|GetIsCurrentCamOffline))
        (Default|ChangeInputType _user_playercontroller "NewEnumerator1")
        (Variables|/Game/Blueprints/FirstPersonController_BP.FirstPersonController_BP_C|SetControlledCamera _user_playercontroller 0)
        (else
          (Default|ClntShowOfflineScreen _user_playercontroller (Variables|Default|GetIsCurrentCamOffline))
          (Default|ClntControlledCameraDestroyed _user_playercontroller))))))

(event Custom|CycleCameras
  (params (CycleUp :type Boolean) (PlayerController :type First%20Person%20Controller%20BP%20Object%20Reference))
  ;[1 1 1] Cycle Cameras
  (if (Networking|IsServer)
    (if CycleUp
      (Utilities|IsValid (Variables|/Game/Cameras/SecurityCamera_BP.SecurityCamera_BP_C|GetSceneCaptureComponent2D (Utilities|Array|Get(acopy) (Variables|Default|GetCamera_BP) (Variables|Default|GetCurrentIndex)))
        (:Is%20Valid
          (Rendering|SetVisibility (Variables|/Game/Cameras/SecurityCamera_BP.SecurityCamera_BP_C|GetSceneCaptureComponent2D (Utilities|Array|Get(acopy) (Variables|Default|GetCamera_BP) (Variables|Default|GetCurrentIndex))) false false))
        (:Is%20Not%20Valid
          _))
      (Math|Integer|IncrementInt (Variables|Default|GetCurrentIndex)
        (:%20%20
          (if (== (Utilities|Array|Length (Variables|Default|GetCamera_BP)) (Variables|Default|GetCurrentIndex))
            (Variables|Default|SetCurrentIndex 0))))
      (else
        (Utilities|IsValid (Variables|/Game/Cameras/SecurityCamera_BP.SecurityCamera_BP_C|GetSceneCaptureComponent2D (Utilities|Array|Get(acopy) (Variables|Default|GetCamera_BP) (Variables|Default|GetCurrentIndex)))
          (:Is%20Valid
            (Rendering|SetVisibility (Variables|/Game/Cameras/SecurityCamera_BP.SecurityCamera_BP_C|GetSceneCaptureComponent2D (Utilities|Array|Get(acopy) (Variables|Default|GetCamera_BP) (Variables|Default|GetCurrentIndex))) false false))
          (:Is%20Not%20Valid
            _))
        (Math|Integer|DecrementInt (Variables|Default|GetCurrentIndex)
          (:%20%20
            (if (< (Variables|Default|GetCurrentIndex) 0)
              (Variables|Default|SetCurrentIndex (- (Utilities|Array|Length (Variables|Default|GetCamera_BP)) 1)))))))
    (if (Variables|/Game/Cameras/SecurityCamera_BP.SecurityCamera_BP_C|GetIsDestroyed (Utilities|Array|Get(acopy) (Variables|Default|GetCamera_BP) (Variables|Default|GetCurrentIndex)))
      (Variables|Default|SetIsCurrentCamOffline true)
      (else
        (Rendering|SetVisibility (Variables|/Game/Cameras/SecurityCamera_BP.SecurityCamera_BP_C|GetSceneCaptureComponent2D (Utilities|Array|Get(acopy) (Variables|Default|GetCamera_BP) (Variables|Default|GetCurrentIndex))) true false)
        (Variables|Default|SetIsCurrentCamOffline false)))
    (if (Pawn|IsLocalPlayerController PlayerController)
      (Default|UpdateCameraName PlayerController (Variables|/Game/Cameras/SecurityCamera_BP.SecurityCamera_BP_C|GetCameraName (Utilities|Array|Get(acopy) (Variables|Default|GetCamera_BP) (Variables|Default|GetCurrentIndex))))
      (Default|ShowOfflineScreen PlayerController (Variables|Default|GetIsCurrentCamOffline))
      (else
        (Default|ClntUpdateCameraName PlayerController (Variables|/Game/Cameras/SecurityCamera_BP.SecurityCamera_BP_C|GetCameraName (Utilities|Array|Get(acopy) (Variables|Default|GetCamera_BP) (Variables|Default|GetCurrentIndex))))
        (Default|ClntShowOfflineScreen PlayerController (Variables|Default|GetIsCurrentCamOffline))))
    (CallFunction|MCSetScreenMaterial (Variables|Default|GetIsCurrentCamOffline))
    (else
      (Development|PrintString "ERROR: Client interaction" true true "(R=1.000000,G=0.000000,B=0.000000,A=1.000000)" 2e+01))))

(event Custom|UI_ShowHint
  (params (PlayerCharacter :type First%20Person%20Character%20Object%20Reference) (Visible :type Boolean))
  ;[1 1 1] UI hint events
  (if (Pawn|IsLocallyControlled PlayerCharacter)
    (Default|UIShowHintInteract PlayerCharacter Visible)
    (else
      (Default|ClntUIShowHint PlayerCharacter Visible))))

(event Custom|UI_ShowAllHints
  (params (Visible :type Boolean))
  ;[1 1 1] UI hint events
  (for _array_element (Variables|Default|GetAllPlayersInTrigger)
    (if (Pawn|IsLocallyControlled _array_element)
      (Default|UIShowHintInteract _array_element Visible)
      (else
        (Default|ClntUIShowHint _array_element Visible)))))

(event Custom|Set_UI_Rendertarget
  (params (UI_render :type Boolean))
  (bind _terminalgroupname (Variables|Default|GetTerminalGroupName))
  (bind _terminalgroupname_2 (Variables|Default|GetTerminalGroupName))
  ;[1 1 1] Switch UI Rendertarget
  (if UI_render
    (Rendering|Material|SetTextureParameterValue (Variables|Default|GetScreenMaterialInstance) "ScreenRenderTexture" (Variables|Default|GetUI_TextureRenderTarget))
    (for _array_element (Variables|Default|GetCamera_BP)
      (if (not (Variables|/Game/Cameras/SecurityCamera_BP.SecurityCamera_BP_C|GetIsDestroyed _array_element))
        (if (Networking|IsServer)
          (Variables|/Script/Engine.SceneCaptureComponent2D|SetTextureTarget (Variables|/Game/Cameras/SecurityCamera_BP.SecurityCamera_BP_C|GetSceneCaptureComponent2D _array_element) (Variables|Default|GetUI_TextureRenderTarget)))))
    ;;[1 0 0] addition for multiple terminals on the same camera-group
    (for _array_element_2 (Variables|Default|GetAllSecurityTerminals)
      (if (Math|Boolean|ANDBoolean (Utilities|Name|Equal(Name) (Variables|SecurityTerminal_BP_C|GetTerminalGroupName _array_element_2) _terminalgroupname_2) (Utilities|Name|NotEqual(Name) _terminalgroupname_2 "None") (!= _array_element_2 self))
        (Rendering|Material|SetTextureParameterValue (Variables|SecurityTerminal_BP_C|GetScreenMaterialInstance _array_element_2) "ScreenRenderTexture" (Variables|SecurityTerminal_BP_C|GetUI_TextureRenderTarget _array_element_2))))
    (else
      (Rendering|Material|SetTextureParameterValue (Variables|Default|GetScreenMaterialInstance) "ScreenRenderTexture" (Variables|Default|GetTextureRenderTarget))
      (for _array_element_3 (Variables|Default|GetCamera_BP)
        (if (not (Variables|/Game/Cameras/SecurityCamera_BP.SecurityCamera_BP_C|GetIsDestroyed _array_element_3))
          (if (Networking|IsServer)
            (Variables|/Script/Engine.SceneCaptureComponent2D|SetTextureTarget (Variables|/Game/Cameras/SecurityCamera_BP.SecurityCamera_BP_C|GetSceneCaptureComponent2D _array_element_3) (Variables|Default|GetTextureRenderTarget)))))
      ;;[1 0 0] addition for multiple terminals on the same camera-group
      (for _array_element_4 (Variables|Default|GetAllSecurityTerminals)
        (if (Math|Boolean|ANDBoolean (Utilities|Name|Equal(Name) (Variables|SecurityTerminal_BP_C|GetTerminalGroupName _array_element_4) _terminalgroupname) (Utilities|Name|NotEqual(Name) _terminalgroupname "None") (!= _array_element_4 self))
          (Rendering|Material|SetTextureParameterValue (Variables|SecurityTerminal_BP_C|GetScreenMaterialInstance _array_element_4) "ScreenRenderTexture" (Variables|SecurityTerminal_BP_C|GetTextureRenderTarget _array_element_4)))))))

(event Custom|DisableAllOtherTerminals
  (params (DisableTerminals :type Boolean))
  ;[1 1 1] Disable all other SecurityTerminals
  (for _array_element (Variables|Default|GetAllSecurityTerminals)
    (if (!= _array_element self)
      (if DisableTerminals
        (Transformation|AddRelativeLocation (Variables|SecurityTerminal_BP_C|GetBox _array_element) "0, 0,-10000.000000" false false)
        (else
          (Transformation|AddRelativeLocation (Variables|SecurityTerminal_BP_C|GetBox _array_element) "0, 0,10000.000000" false false))))))

(event EventBeginPlay
  ;[1 1 1] BeginPlay
  (if (Networking|IsServer)
    (Rendering|SetVisibility (Variables|/Game/Cameras/SecurityCamera_BP.SecurityCamera_BP_C|GetSceneCaptureComponent2D (Utilities|Array|Get(acopy) (Variables|Default|GetCamera_BP) (Variables|Default|GetCurrentIndex))) true false)
    (for _array_element (Variables|Default|GetCamera_BP)
      (Variables|/Game/Cameras/SecurityCamera_BP.SecurityCamera_BP_C|SetOwningTerminal _array_element self))
    (bind _outactors (Actor|GetAllActorsOfClass "SecurityTerminal_BP_C"))
    (Variables|Default|SetAllSecurityTerminals _outactors)))

(event EventInteractwithActor
  (params (UserController :type First%20Person%20Controller%20BP%20Object%20Reference))
  (bind _camera_bp (Variables|Default|GetCamera_BP))
  (bind _currentindex (Variables|Default|GetCurrentIndex))
  (bind _output (Utilities|Array|Get(acopy) _camera_bp _currentindex))
  (bind _cameraname (Variables|/Game/Cameras/SecurityCamera_BP.SecurityCamera_BP_C|GetCameraName _output))
  ;[1 1 1] Event Interact
  (if (Networking|IsServer)
    (if (not (Variables|Default|GetIsInUse))
      (Variables|Default|SetUser_PlayerController UserController)
      (Variables|Default|SetIsInUse true)
      (CallFunction|UIShowAllHints false)
      (CallFunction|DisableAllOtherTerminals true)
      (if (Variables|/Game/Cameras/SecurityCamera_BP.SecurityCamera_BP_C|GetIsDestroyed (Utilities|Array|Get(acopy) (Variables|Default|GetCamera_BP) (Variables|Default|GetCurrentIndex)))
        (Variables|Default|SetIsCurrentCamOffline true)
        (CallFunction|MCSetScreenMaterial true)
        (else
          (Variables|Default|SetIsCurrentCamOffline false)
          (CallFunction|MCSetScreenMaterial false)))
      (CallFunction|SetUIRendertarget true)
      (if (Pawn|IsLocalPlayerController UserController)
        (Variables|/Game/Blueprints/FirstPersonController_BP.FirstPersonController_BP_C|SetSecurityTerminal UserController self)
        (Default|ShowSecurityScreenWB UserController true)
        (Default|UpdateCameraName UserController _cameraname)
        (Default|ShowOfflineScreen UserController (Variables|Default|GetIsCurrentCamOffline))
        (else
          (Default|ClntShowSecurityScreen UserController true self)
          (Default|ClntUpdateCameraName UserController _cameraname)
          (Default|ClntShowOfflineScreen UserController (Variables|Default|GetIsCurrentCamOffline)))))
    (else
      (Development|PrintString "ERROR: Client interaction" true true "(R=1.000000,G=0.000000,B=0.000000,A=1.000000)" 2e+01))))

(fn ConstructionScript
  (bind _returnvalue (Rendering|Material|CreateDynamicMaterialInstance (Variables|Default|GetCube) 0 0 "None" :!class /Script/Engine.PrimitiveComponent))
  (Variables|Default|SetScreenMaterialInstance _returnvalue)
  (Rendering|Material|SetTextureParameterValue _returnvalue "ScreenRenderTexture" (Variables|Default|GetTextureRenderTarget)))